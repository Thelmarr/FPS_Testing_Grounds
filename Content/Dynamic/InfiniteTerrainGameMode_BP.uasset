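; Game mode for an infinite terrain game that lays down tiles end to end and keeps the score.
; On BeginPlay it calls PopulateBoundsVolumePool, which is defined outside these graphs, then spawns the initial tiles.
; SpawnTile places a Tile_BP at NextTileTransform and stores that tile's attach location as the next transform, forming a chain.
; UpdateScore increments the score and GetScore returns it.
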(event `self.ReceiveBeginPlay`
  (`self.PopulateBoundsVolumePool`)
  (for _ (range 2)
    (`self.Spawn Tile`)))

(fn `Get_Score`
  (returns (Score :type Integer))
  (return (`self.Score`)))

(fn `Spawn Tile`
  (bind _returnvalue (`|SpawnActorFromClass` "/Game/Dynamic/Terrain/Tile_BP.Tile_BP_C" (`self.Next Tile Transform`) "Undefined" "OverrideRootScale" null null))
  (bind _attach_transform (`/Game/Dynamic/Terrain/Tile_BP.Get Attach Location` _returnvalue))
  (set `self.Next Tile Transform` _attach_transform))

(fn `Update Score`
  (`/Engine/EditorBlueprintResources/StandardMacros.IncrementInt` (`self.Score`)))

(fn `UserConstructionScript`)